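; Player ship pawn for the space shooter, handling movement and firing through Enhanced Input.
; BeginPlay adds the ship's mapping context, and the move action stores a 2D input that is cleared on cancel or completion.
; Tick moves the ship along its right and forward vectors by that input and Speed, with sweep.
; Fire spawns Ammo at FirePoint, gated by a CanFire flag that a FireDelay timer restores.
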(event `self.ReceiveBeginPlay`
  ; Setup Enhance Input
  (bind _asplayer_controller (cast `PlayerController` (`self.GetController`)))
  (bind _returnvalue (pcsubsystem `EnhancedInputLocalPlayerSubsystem` _asplayer_controller))
  (`/Engine/EditorBlueprintResources/StandardMacros.IsValid` _returnvalue
    (:`Is Valid`
      (`EnhancedInputSubsystemInterface.AddMappingContext` _returnvalue "/Game/SpaceShooter/Input/IAM_Input_MyShip_Mapping.IAM_Input_MyShip_Mapping" 0 (struct)))))

(event `self.ReceiveTick`
  (params (DeltaSeconds :type "Float (single-precision)"))
  (bind (_inputsaved_x _inputsaved_y) (`KismetMathLibrary.BreakVector2D` (`self.InputSaved`)))
  (bind _returnvalue (* DeltaSeconds (`self.Speed`)))
  ; Update Possition
  (`self.K2_SetActorLocation` (+ (`self.K2_GetActorLocation`) (+ (* (`self.GetActorRightVector`) (* _returnvalue _inputsaved_x)) (* (* _returnvalue _inputsaved_y) (`self.GetActorForwardVector`)))) true))

(event `EnhancedInput|/Game/SpaceShooter/Input/IA_Input_MyFire`
  (params (ActionValue :type Boolean) (ElapsedSeconds :type "Float (double-precision)") (TriggeredSeconds :type "Float (double-precision)") (InputAction :type "InputAction Object Reference" :default "/Game/SpaceShooter/Input/IA_Input_MyFire.IA_Input_MyFire"))
  ; Shooter Logic
  (:`Triggered`
    (if (`self.CanFire`)
      (`self.DoFire`)
      (set `self.CanFire` false)
      (`KismetSystemLibrary.K2_SetTimerDelegate` (delegate `RestoreFire`) (`self.FireDelay`)))))

(event `RestoreFire`
  ; Shooter Logic
  (set `self.CanFire` true))

(event `EnhancedInput|/Game/SpaceShooter/Input/IA_Input_MyMove`
  (params (ActionValue :type "Vector2D Structure") (ElapsedSeconds :type "Float (double-precision)") (TriggeredSeconds :type "Float (double-precision)") (InputAction :type "InputAction Object Reference" :default "/Game/SpaceShooter/Input/IA_Input_MyMove.IA_Input_MyMove"))
  ; Move Logic
  (:`Triggered`
    (set `self.InputSaved` ActionValue))
  (:`Canceled`
    (set `self.InputSaved` (0.0 0.0) :!label _label))
  (:`Completed`
    (goto _label)))

(fn `DoFire`
  ; DoFire MyShip Function
  (`|SpawnActorFromClass` (`self.Ammo`) (`SceneComponent.K2_GetComponentToWorld` (`self.FirePoint`)) "Undefined" "MultiplyWithRoot" null null))

(fn `UserConstructionScript`)