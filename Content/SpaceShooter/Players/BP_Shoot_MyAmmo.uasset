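; BP_Shoot_MyAmmo is the player's bullet in the space shooter, playing a sound when it spawns.
; Tick moves it along its forward vector by Speed plus DeltaSeconds, added rather than multiplied, without sweep.
; Overlapping an "External" actor destroys it immediately.
; An "Enemy" overlap triggers explosion effects and destroys it a second later; the intended hide passes false, leaving it visible meanwhile.
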(event `self.ReceiveBeginPlay`
  ; Bullet Begin
  (`GameplayStatics.PlaySound2D` "/Engine/VREditor/Sounds/UI/Click_on_Button.Click_on_Button" 0.5 1.0 0.0 null null))

(event `self.ReceiveActorBeginOverlap`
  (params (OtherActor :type "Actor Object Reference"))
  (bind _tags (`Actor.Tags` OtherActor))
  ; Bullet End
  (if (`KismetArrayLibrary.Array_Contains` _tags "External")
    (`self.K2_DestroyActor`)
    (elif (`KismetArrayLibrary.Array_Contains` _tags "Enemy")
      (`self.FXKilledAmmoPlayer`)
      (`KismetSystemLibrary.Delay` 1.0)
      (`self.K2_DestroyActor`))))

(event `self.ReceiveTick`
  (params (DeltaSeconds :type "Float (single-precision)"))
  ; Bullet Movement
  (`self.K2_SetActorLocation` (+ (`self.K2_GetActorLocation`) (* (`self.GetActorForwardVector`) (+ DeltaSeconds (`self.Speed`))))))

(fn `FXKilledAmmoPlayer`
  ; Killed Player Ammo Sound FX and Hidden (Not Destroyed)
  (`GameplayStatics.SpawnEmitterAtLocation` "/Game/StarterContent/Particles/P_Explosion.P_Explosion" (`self.K2_GetActorLocation`))
  (`GameplayStatics.PlaySound2D` "/Game/StarterContent/Audio/Explosion02.Explosion02" 0.35 1.0 0.0 null null)
  (`self.SetActorHiddenInGame` false))

(fn `UserConstructionScript`)