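; Player ship pawn for the space shooter, handling movement, firing, damage and death.
; Enhanced Input saves a movement vector that Tick applies as swept, speed-scaled offsets, while TryFire spawns ammo at FirePoint behind a timer-reset cooldown.
; Overlapping an Enemy-tagged actor damages that enemy.
; PlayerHealthImpact reduces health and at zero plays explosion effects, tells BP_GameMode to subtract a life and destroys the pawn.
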(event `self.ReceiveBeginPlay`
  ; Setup Enhance Input
  (set `self.Lifes` 3)
  (set `self.Bombs` 1)
  (bind _asplayer_controller (cast `PlayerController` (`self.GetController`)))
  (bind _returnvalue (pcsubsystem `EnhancedInputLocalPlayerSubsystem` _asplayer_controller))
  (`/Engine/EditorBlueprintResources/StandardMacros.IsValid` _returnvalue
    (:`Is Valid`
      (`EnhancedInputSubsystemInterface.AddMappingContext` _returnvalue "/Game/SpaceShooter/Input/IAM_Input_MyShip_Mapping.IAM_Input_MyShip_Mapping" 0 (struct))
      (add `self.OnPawnDestroy` (delegate `PawnDestroyed_Event`)))))

(event `PawnDestroyed_Event`
  ; Setup Enhance Input
  (`KismetSystemLibrary.Delay` 0.1)
  (`GameplayStatics.PlaySound2D` "/Game/StarterContent/Audio/Explosion02.Explosion02" 0.35 1.0 0.0 null null)
  (`KismetSystemLibrary.Delay` 0.1)
  (`GameplayStatics.SpawnEmitterAtLocation` "/Game/StarterContent/Particles/P_Explosion.P_Explosion" (`self.K2_GetActorLocation`))
  (`GameplayStatics.PlaySound2D` "/Game/StarterContent/Audio/Explosion02.Explosion02" 0.35 1.0 0.0 null null)
  (`KismetSystemLibrary.Delay` 0.2)
  (`self.K2_DestroyActor`))

(event `self.ReceiveTick`
  (params (DeltaSeconds :type "Float (single-precision)"))
  (bind (_inputsaved_x _inputsaved_y) (`KismetMathLibrary.BreakVector2D` (`self.InputSaved`)))
  (bind _inputsaved_x_2 (`KismetMathLibrary.BreakVector2D` (`self.InputSaved`)))
  ; Update Possition
  (`self.K2_SetActorLocation` (+ (* (`self.GetActorRightVector`) (* (* DeltaSeconds (`self.Speed`)) _inputsaved_x_2)) (`self.K2_GetActorLocation`)) true)
  (`self.K2_SetActorLocation` (+ (* (* (* DeltaSeconds (`self.Speed`)) _inputsaved_y) (`self.GetActorForwardVector`)) (`self.K2_GetActorLocation`)) true))

(event `EnhancedInput|/Game/SpaceShooter/Input/IA_Input_MyMove`
  (params (ActionValue :type "Vector2D Structure") (ElapsedSeconds :type "Float (double-precision)") (TriggeredSeconds :type "Float (double-precision)") (InputAction :type "InputAction Object Reference" :default "/Game/SpaceShooter/Input/IA_Input_MyMove.IA_Input_MyMove"))
  ; Move Logic
  (:`Triggered`
    (set `self.InputSaved` ActionValue))
  (:`Canceled`
    (set `self.InputSaved` (0.0 0.0) :!label _label))
  (:`Completed`
    (goto _label)))

(event `PlayerHealthImpact`
  (params (HealthImpact :type Integer))
  ; Player recibe hits hasta que muere, entonces llama al Game Mode para decir qué hacer (en función de las vidas que tenga)
  (bind _output_get (set `self.Health` (- (`self.Health`) HealthImpact)))
  (if (<= _output_get 0)
    (`self.SetActorHiddenInGame` false)
    (`self.PlayerDestructionFX`)
    (bind _asbp_game_mode (cast `/Game/SpaceShooter/BP_GameMode` (`GameplayStatics.GetGameMode`)))
    (`/Game/SpaceShooter/BP_GameMode.SubstractLive` _asbp_game_mode)
    (`KismetSystemLibrary.Delay` 0.2)
    (`self.K2_DestroyActor`)))

(event `TryFire`
  ; Mira si puede o no puede disparar la nave
  (if (`self.CanFire`)
    (`self.Fire`)
    (set `self.CanFire` false)
    (`KismetSystemLibrary.K2_SetTimerDelegate` (delegate `CustomEvent`) (`self.FireDelay`))))

(event `CustomEvent`
  ; Mira si puede o no puede disparar la nave
  (set `self.CanFire` true))

(event `self.ReceiveActorBeginOverlap`
  (params (OtherActor :type "Actor Object Reference"))
  ; Sólo tiene que saber si un Enemy se ha chocado con él, en cuyo caso le hará un daño
  (`/Engine/EditorBlueprintResources/StandardMacros.IsValid` OtherActor
    (:`Is Valid`
      (if (`KismetArrayLibrary.Array_Contains` (`Actor.Tags` OtherActor) "Enemy")
        (bind _asbp_base_my_enemy (cast `/Game/SpaceShooter/Enemies/BP_Base_MyEnemy` OtherActor))
        (`/Engine/EditorBlueprintResources/StandardMacros.IsValid` _asbp_base_my_enemy
          (:`Is Valid`
            (`/Game/SpaceShooter/Enemies/BP_Base_MyEnemy.EnemyHitted` _asbp_base_my_enemy (`self.Health Hitted`))))))))

(fn `Fire`
  ; Fire MyShip2 Function
  (`|SpawnActorFromClass` (`self.PawnAmmo`) (`SceneComponent.K2_GetComponentToWorld` (`self.FirePoint`)) "Undefined" "MultiplyWithRoot" null null))

(fn `PlayerDestructionFX`
  ; Player Destruction FX and Sound
  (`GameplayStatics.SpawnEmitterAtLocation` "/Game/StarterContent/Particles/P_Explosion.P_Explosion" (`self.K2_GetActorLocation`))
  (`GameplayStatics.PlaySound2D` "/Game/StarterContent/Audio/Explosion02.Explosion02" 0.35 1.0 0.0 null null)
  (`self.SetActorHiddenInGame` false))

(fn `UserConstructionScript`)