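; Space shooter game mode that tracks points, lives, bombs and health, initialised on BeginPlay along with the player start transform and camera.
; EnemyDestroyed adds points; PlayerHitted subtracts health and calls PlayerDestroyed at zero or below.
; PlayerDestroyed respawns and possesses a new pawn after a delay while lives remain, otherwise reloads the level.
; Points and lives reach the HUD widget through BP_PlayerController and BP_HUD; the bombs update is never run.
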(event `self.ReceiveBeginPlay`
  ; Begin Play - Set Init Global Variables
  (set `self.Points` 0)
  (`self.SetHUDPoints`)
  (set `self.Lives` 3)
  (`self.SetHUDLives`)
  (set `self.Bombs` 1)
  (set `self.Health` 100)
  (`self.InitPlayer`)
  (`self.InitCameraActor`))

(event `EnemyDestroyed`
  (params (Points :type Integer))
  ; Enemigo destruido sumo sus puntos
  (set `self.Points` (+ Points (`self.Points`)))
  (`self.SetHUDPoints`))

(event `PlayerDestroyed`
  (bind _returnvalue (- (`self.Lives`) 1))
  ; Jugador destruido miro si hay vidas, si las hay respawn, sino restart
  (if (>= _returnvalue 1)
    (set `self.Lives` _returnvalue)
    (`KismetSystemLibrary.Delay` (`self.RespawnDelay`))
    (`self.RespawnPlayer`)
    (`self.SetHUDLives`)
    (else
      (bind _returnvalue_2 (`GameplayStatics.GetCurrentLevelName` true))
      (`GameplayStatics.OpenLevel` (`KismetStringLibrary.Conv_StringToName` _returnvalue_2)))))

(event `PlayerHitted`
  (params (HealthHitted :type Integer))
  ; Quito la vida del impacto, cuando sea 0 o menor de 0 se habrá perdido una vida, por lo que llamo a PlayerDestroyed
  (bind _output_get (set `self.Health` (- (`self.Health`) HealthHitted)))
  (if (<= _output_get 0)
    (`KismetSystemLibrary.PrintString` "[byGamePlayer] Nave Destruida" true true (struct :`G` 0.66 :`B` 1.0 :`A` 1.0) 20.0)
    (`self.PlayerDestroyed`)))

(event `self.ReceiveActorOnClicked`
  (params (ButtonPressed :type "Key Structure")))

(fn `InitCameraActor`
  ; Obtiene la información de la Cámara, para mantenerla continua durante el juego
  (bind _outactors (`GameplayStatics.GetAllActorsOfClass` "/Script/Engine.CameraActor"))
  (set `self.MainCamera` (`|GetArrayItem` _outactors)))

(fn `InitPlayer`
  (bind _returnvalue (`GameplayStatics.GetPlayerPawn` 0))
  ; Inicializa el Player obteniendo primero su posición inicial (para hacer respawn luego)
  (`/Engine/EditorBlueprintResources/StandardMacros.IsValid` _returnvalue
    (:`Is Valid`
      (set `self.PlayerBeginTransform` (`self.GetTransform` _returnvalue)))))

(fn `RespawnPlayer`
  ; RespawnPlayer Function
  (bind _returnvalue (`|SpawnActorFromClass` (`self.PlayerPawnClass`) (`self.PlayerBeginTransform`) "Undefined" "MultiplyWithRoot" null null))
  (`Controller.Possess` (`GameplayStatics.GetPlayerController` 0) _returnvalue))

(fn `SetHUDBombs`
  (bind _returnvalue (`GameplayStatics.GetPlayerController` 0))
  (cast `/Game/SpaceShooter/BP_PlayerController` (`GameplayStatics.GetPlayerController` 0))
  (`/Engine/EditorBlueprintResources/StandardMacros.IsValid` _returnvalue
    (:`Is Valid`
      (bind _asbp_player_controller (cast `/Game/SpaceShooter/BP_PlayerController` _returnvalue))
      (bind _returnvalue_2 (`PlayerController.GetHUD` _asbp_player_controller))
      (`/Engine/EditorBlueprintResources/StandardMacros.IsValid` _returnvalue_2
        (:`Is Valid`
          (bind _asbp_hud (cast `/Game/SpaceShooter/HUD/BP_HUD` _returnvalue_2))
          (bind _hudwidget (`/Game/SpaceShooter/HUD/BP_HUD.HUDWidget` _asbp_hud))
          (`/Engine/EditorBlueprintResources/StandardMacros.IsValid` _hudwidget
            (:`Is Valid`
              (`/Game/SpaceShooter/HUD/BP_Widget.UpdateBombs` _hudwidget (`self.Bombs`)))))))))

(fn `SetHUDLives`
  (bind _returnvalue (`GameplayStatics.GetPlayerController` 0))
  (cast `/Game/SpaceShooter/BP_PlayerController` (`GameplayStatics.GetPlayerController` 0))
  (`/Engine/EditorBlueprintResources/StandardMacros.IsValid` _returnvalue
    (:`Is Valid`
      (bind _asbp_player_controller (cast `/Game/SpaceShooter/BP_PlayerController` _returnvalue))
      (bind _returnvalue_2 (`PlayerController.GetHUD` _asbp_player_controller))
      (`/Engine/EditorBlueprintResources/StandardMacros.IsValid` _returnvalue_2
        (:`Is Valid`
          (bind _asbp_hud (cast `/Game/SpaceShooter/HUD/BP_HUD` _returnvalue_2))
          (bind _hudwidget (`/Game/SpaceShooter/HUD/BP_HUD.HUDWidget` _asbp_hud))
          (`/Engine/EditorBlueprintResources/StandardMacros.IsValid` _hudwidget
            (:`Is Valid`
              (`/Game/SpaceShooter/HUD/BP_Widget.UpdateLifes` _hudwidget (`self.Lives`)))))))))

(fn `SetHUDPoints`
  (bind _returnvalue (`GameplayStatics.GetPlayerController` 0))
  (cast `/Game/SpaceShooter/BP_PlayerController` (`GameplayStatics.GetPlayerController` 0))
  (`/Engine/EditorBlueprintResources/StandardMacros.IsValid` _returnvalue
    (:`Is Valid`
      (bind _asbp_player_controller (cast `/Game/SpaceShooter/BP_PlayerController` _returnvalue))
      (bind _returnvalue_2 (`PlayerController.GetHUD` _asbp_player_controller))
      (`/Engine/EditorBlueprintResources/StandardMacros.IsValid` _returnvalue_2
        (:`Is Valid`
          (bind _asbp_hud (cast `/Game/SpaceShooter/HUD/BP_HUD` _returnvalue_2))
          (bind _hudwidget (`/Game/SpaceShooter/HUD/BP_HUD.HUDWidget` _asbp_hud))
          (`/Engine/EditorBlueprintResources/StandardMacros.IsValid` _hudwidget
            (:`Is Valid`
              (`/Game/SpaceShooter/HUD/BP_Widget.UpdatePoints` _hudwidget (`self.Points`)))))))))

(fn `UserConstructionScript`)