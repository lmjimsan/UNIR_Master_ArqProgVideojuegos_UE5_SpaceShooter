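; Player controller for the space shooter that owns the game state: start screen, gameplay and game over.
; BeginPlay adds the ship input mapping, caches the ship pawn and HUD, and sets the first CameraActor as view target.
; The fire action either shoots or advances the state, depending on the current one.
; SetGameState switches input mode, cursor and pawn input, then updates the HUD, using the gameplay view for start screen too.
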(event `self.ReceiveBeginPlay`
  ; Inicio del Player Controller donde fijamos la cámara principal a este objeto (no al GameMode)
  (`EnhancedInputSubsystemInterface.AddMappingContext` (pcsubsystem `EnhancedInputLocalPlayerSubsystem` (`GameplayStatics.GetPlayerController` 0)) "/Game/SpaceShooter/Input/IAM_Input_MyShip_Mapping.IAM_Input_MyShip_Mapping" 0 (struct))
  (bind _asbp_pawn_my_ship_2 (cast `/Game/SpaceShooter/Players/BP_Pawn_MyShip2` (`GameplayStatics.GetPlayerPawn` 0)))
  (set `self.As BP Pawn My Ship 2` _asbp_pawn_my_ship_2)
  (bind _asbp_hud (cast `/Game/SpaceShooter/HUD/BP_HUD` (`self.GetHUD`)))
  (set `self.As BP HUD` _asbp_hud)
  (bind _outactors (`GameplayStatics.GetAllActorsOfClass` "/Script/Engine.CameraActor"))
  (bind _output (`|GetArrayItem` _outactors))
  (`/Engine/EditorBlueprintResources/StandardMacros.IsValid` _output
    (:`Is Valid`
      (set `self.MainCamera` _output)
      (`self.SetViewTargetWithBlend` (`self.MainCamera`)))))

(event `EnhancedInput|/Game/SpaceShooter/Input/IA_Input_MyFire`
  (params (ActionValue :type Boolean) (ElapsedSeconds :type "Float (double-precision)") (TriggeredSeconds :type "Float (double-precision)") (InputAction :type "InputAction Object Reference" :default "/Game/SpaceShooter/Input/IA_Input_MyFire.IA_Input_MyFire"))
  (:`Triggered`
    (switch `/Game/SpaceShooter/enumGameWay` (`self.CurrentGameState`)
      (:`NewEnumerator0`
        (`self.SetGameState` "NewEnumerator1"))
      (:`NewEnumerator1`
        (`/Engine/EditorBlueprintResources/StandardMacros.IsValid` (`self.As BP Pawn My Ship 2`)
          (:`Is Valid`
            (`/Game/SpaceShooter/Players/BP_Pawn_MyShip2.TryFire` (`self.As BP Pawn My Ship 2`)))
          (:`Is Not Valid`
            (bind _asbp_pawn_my_ship_2 (cast `/Game/SpaceShooter/Players/BP_Pawn_MyShip2` (`self.K2_GetPawn`)))
            (`/Game/SpaceShooter/Players/BP_Pawn_MyShip2.TryFire` _asbp_pawn_my_ship_2))))
      (:`NewEnumerator2`
        (`self.SetGameState` "NewEnumerator0")))))

(event `self.ReceivePossess`
  (params (PossessedPawn :type "Pawn Object Reference"))
  (bind _asbp_pawn_my_ship_2 (cast `/Game/SpaceShooter/Players/BP_Pawn_MyShip2` (`GameplayStatics.GetPlayerPawn` 0)))
  (set `self.As BP Pawn My Ship 2` _asbp_pawn_my_ship_2))

(event `self.ReceiveUnPossess`
  (params (UnpossessedPawn :type "Pawn Object Reference"))
  (set `self.As BP Pawn My Ship 2` null))

(fn `SetGameState`
  (params (NewState :type "/Game/SpaceShooter/enumGameWay Enum" :default "NewEnumerator0"))
  (bind _as_bp_hud (`self.As BP HUD`))
  (bind _as_bp_hud_2 (`self.As BP HUD`))
  (bind _as_bp_hud_3 (`self.As BP HUD`))
  (bind _output_get (set `self.CurrentGameState` NewState))
  (`KismetSystemLibrary.PrintString` "SetGameState: [NewState]")
  (switch `/Game/SpaceShooter/enumGameWay` _output_get
    (:`NewEnumerator0`
      (`WidgetBlueprintLibrary.SetInputMode_GameAndUIEx` self null)
      (set `self.bShowMouseCursor` true)
      (`self.DisableInput` (`self.As BP Pawn My Ship 2`) null)
      (`/Engine/EditorBlueprintResources/StandardMacros.IsValid` _as_bp_hud_3
        (:`Is Valid`
          (`/Game/SpaceShooter/HUD/BP_HUD.ShowGamePlay` _as_bp_hud_3))
        (:`Is Not Valid`
          (`KismetSystemLibrary.PrintString` "[BP_PlayerController:SetGameState] HUD Widget No listo" true true (struct :`G` 0.66 :`B` 1.0 :`A` 1.0) 20.0 :!label _label))))
    (:`NewEnumerator1`
      (`WidgetBlueprintLibrary.SetInputMode_GameOnly` self)
      (set `self.bShowMouseCursor` false)
      (`self.EnableInput` (`self.As BP Pawn My Ship 2`) null)
      (`/Engine/EditorBlueprintResources/StandardMacros.IsValid` _as_bp_hud
        (:`Is Valid`
          (`/Game/SpaceShooter/HUD/BP_HUD.ShowGamePlay` _as_bp_hud))
        (:`Is Not Valid`
          (goto _label))))
    (:`NewEnumerator2`
      (`WidgetBlueprintLibrary.SetInputMode_GameAndUIEx` self null)
      (set `self.bShowMouseCursor` true)
      (`self.DisableInput` (`self.As BP Pawn My Ship 2`) null)
      (`/Engine/EditorBlueprintResources/StandardMacros.IsValid` _as_bp_hud_2
        (:`Is Valid`
          (`/Game/SpaceShooter/HUD/BP_HUD.ShowGameOver` _as_bp_hud_2))
        (:`Is Not Valid`
          (goto _label))))))

(fn `UserConstructionScript`)