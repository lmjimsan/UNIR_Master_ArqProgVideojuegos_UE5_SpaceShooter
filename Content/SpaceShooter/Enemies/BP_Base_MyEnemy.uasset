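; Base enemy for the space shooter that flies straight, shoots, takes damage and hurts the player on contact.
; Tick moves it along the forward vector cached at BeginPlay and spawns ammo from FirePoint on a re-randomized interval.
; EnemyHitted subtracts health; at zero it awards points through BP_GameMode, plays explosion effects and destroys itself after a short delay.
; Overlapping a Player-tagged actor damages the BP_Pawn_MyShip2 player pawn without destroying the enemy.
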(event `self.ReceiveBeginPlay`
  (bind _delayshoot (`self.DelayShoot`))
  ; Enemy Begin
  (set `self.RandomDelayShoot` (`KismetMathLibrary.RandomFloatInRange` _delayshoot (+ _delayshoot 2.0)))
  (set `self.MovementVector` (`self.GetActorForwardVector`)))

(event `EnemyHitted`
  (params (HealthHitted :type Integer))
  ; Enemy Hitted
  (bind _output_get (set `self.EnemyHealth` (- (`self.EnemyHealth`) HealthHitted)))
  (if (<= _output_get 0)
    (`self.GivePointsToPlayer`)
    (`self.SetActorHiddenInGame` false)
    (`self.EnemyDestructionFX`)
    (`KismetSystemLibrary.Delay` 0.2)
    (`self.K2_DestroyActor`)))

(event `self.ReceiveTick`
  (params (DeltaSeconds :type "Float (single-precision)"))
  (bind _delayshoot (`self.DelayShoot`))
  ; Enemy Movement and Fire
  (`self.Movimiento` DeltaSeconds)
  (bind _output_get (set `self.ShootCurrentTime` (+ DeltaSeconds (`self.ShootCurrentTime`))))
  (if (> _output_get (`self.RandomDelayShoot`))
    (set `self.RandomDelayShoot` (`KismetMathLibrary.RandomFloatInRange` _delayshoot (+ _delayshoot 2.0)))
    (set `self.ShootCurrentTime` 0.0)
    (`self.Fire`)))

(event `self.ReceiveActorBeginOverlap`
  (params (OtherActor :type "Actor Object Reference"))
  ; Sólo tiene que saber si el Player se ha chocado con él, en cuyo caso le hará un daño
  (`/Engine/EditorBlueprintResources/StandardMacros.IsValid` OtherActor
    (:`Is Valid`
      (if (`KismetArrayLibrary.Array_Contains` (`Actor.Tags` OtherActor) "Player")
        (`self.HitHealthToPlayer`)))))

(fn `EnemyDestructionFX`
  ; Enemy Destruction FX and Sound
  (`GameplayStatics.SpawnEmitterAtLocation` "/Game/StarterContent/Particles/P_Explosion.P_Explosion" (`self.K2_GetActorLocation`))
  (`GameplayStatics.PlaySound2D` "/Game/StarterContent/Audio/Explosion02.Explosion02" 0.35 1.0 0.0 null null))

(fn `Fire`
  ; Fire Function
  (bind _returnvalue (`|SpawnActorFromClass` (`self.EnemyAmmo`) (`SceneComponent.K2_GetComponentToWorld` (`self.FirePoint`)) "Undefined" "MultiplyWithRoot" null null))
  (`/Engine/EditorBlueprintResources/StandardMacros.IsValid` _returnvalue
    (:`Is Valid`
      (`self.K2_SetActorRotation` _returnvalue (`self.K2_GetActorRotation`) false))))

(fn `GivePointsToPlayer`
  (bind _returnvalue (`GameplayStatics.GetGameMode`))
  ; Sube los puntos a Game Mode para que además de guardarlos los sume al HUD
  (`/Engine/EditorBlueprintResources/StandardMacros.IsValid` _returnvalue
    (:`Is Valid`
      (bind _asbp_game_mode (cast `/Game/SpaceShooter/BP_GameMode` _returnvalue))
      (`/Game/SpaceShooter/BP_GameMode.EnemyGivePointsToPlayer` _asbp_game_mode (`self.EnemyPoints`)))))

(fn `HitHealthToPlayer`
  (bind _returnvalue (`GameplayStatics.GetPlayerPawn` 0))
  ; Hit Health To Player
  (`/Engine/EditorBlueprintResources/StandardMacros.IsValid` _returnvalue
    (:`Is Valid`
      (bind _asbp_pawn_my_ship_2 (cast `/Game/SpaceShooter/Players/BP_Pawn_MyShip2` _returnvalue))
      (`/Game/SpaceShooter/Players/BP_Pawn_MyShip2.PlayerHealthImpact` _asbp_pawn_my_ship_2 (`self.Health Hitted`)))))

(fn `Movimiento`
  (params (DeltaTime :type "Float (double-precision)"))
  ; Movement Function
  (`self.K2_SetActorLocation` (+ (`self.K2_GetActorLocation`) (* (* DeltaTime (`self.Speed`)) (`self.MovementVector`)))))

(fn `UserConstructionScript`)